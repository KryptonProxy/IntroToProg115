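; Pickup actor that, on PickUpItem, flies into the player's backpack and adds health.
; Its mesh, material, value and displayed name come from a data table row keyed by the Type enum, applied in the construction script and on BeginPlay.
; A timeline shrinks, spins and moves it to the backpack with collision off, then triggers the player's backpack effect and destroys the actor.
; Health gain is a fixed amount, independent of Value.
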(event EventBeginPlay
  ;[1 1 1] BeginPlay
  (bind _returnvalue (Utilities|GetDataTableRow "/Game/Item/NewDataTable.NewDataTable" (Utilities|String|StringToName (Utilities|String|EnumtoString (Variables|Default|GetType))))
    (:then
      (CallFunction|SetProperty _returnvalue))))

(event EventPickUpItem
  (params (Player :type Third%20Person%20Character%20Soft%20Object%20Reference))
  ;[1 1 1] Pickup Anim
  (Variables|Default|SetPlayer Player)
  (Utilities|PreparePickup)
  (bind _lerpalpha (Timeline|PIckupAnimation PlayFromStart)
    (:Update
      (CallFunction|PlayAnimation _lerpalpha (Utilities|ResolveSoftReference (Variables|Default|GetPlayer))))
    (:Finished
      (Actor|DestroyActor)
      (Default|PlayBackpackEffect (Utilities|ResolveSoftReference (Variables|Default|GetPlayer)) "/Game/StarterContent/Particles/P_Explosion.P_Explosion" "/Game/StarterContent/Audio/Explosion02.Explosion02")
      (Utilities|AddHealth 1))))

(event EventTick
  (params (DeltaSeconds :type Float%20%28single-precision%29)))

(fn ConstructionScript
  (bind _returnvalue (Utilities|GetDataTableRow "/Game/Item/NewDataTable.NewDataTable" (Utilities|String|StringToName (Utilities|String|EnumtoString (Variables|Default|GetType))))
    (:then
      (CallFunction|SetProperty _returnvalue))))

(fn NewFunction0
  (params (NewMesh :type Static%20Mesh%20Object%20Reference) (Material :type Material%20Interface%20Object%20Reference))
  (Components|StaticMesh|SetStaticMesh (Variables|Default|GetStaticMesh) NewMesh)
  (Rendering|Material|SetMaterial (Variables|Default|GetStaticMesh) 0 Material))

(fn SetProperty
  (params (PickUp :type Pick%20Up%20Structure%20%28by%20ref%29))
  (bind (_name _mesh _material _value) (Utilities|Struct|BreakPickUp PickUp))
  (bind _staticmesh (Variables|Default|GetStaticMesh))
  (Components|StaticMesh|SetStaticMesh _staticmesh _mesh)
  (Rendering|Material|SetMaterial _staticmesh 0 _material)
  (Variables|Default|SetValue _value)
  (Rendering|Components|TextRender|SetText (Variables|Default|GetName) (Utilities|Text|ToText(Name) _name))
  ;[1 1 1] Change the name of widget
  (bind _asname (Utilities|Casting|CastToName (UserInterface|GetUserWidgetObject (Variables|Default|GetWidget))))
  (Variables|/Game/Item/Name.Name_C|SetName _asname (Utilities|String|ToString(Name) _name)))

(fn PlayAnimation
  (params (LerpAlpha :type Float%20%28single-precision%29) (Player :type Third%20Person%20Character%20Object%20Reference))
  (bind _returnvalue (* 1e+02 LerpAlpha))
  (Utilities|FlowControl|Sequence
    (:then_0
      (Transformation|SetWorldScale3D (Variables|Default|GetStaticMesh) (Math|Vector|Lerp(Vector) "1.000000,1.000000,1.000000" "0, 0, 0" LerpAlpha)))
    (:then_1
      (Transformation|SetActorLocation (Math|Vector|Lerp(Vector) (Variables|Default|GetSetLocation) (- (Transformation|GetWorldLocation (Variables|/Game/ThirdPersonCPP/Blueprints/ThirdPersonCharacter.ThirdPersonCharacter_C|GetBackpack Player)) "0, 0,50.000000") LerpAlpha) true false))
    (:then_2
      (Transformation|AddWorldRotation (Variables|Default|GetStaticMesh) (Math|Rotator|MakeRotator _returnvalue _returnvalue _returnvalue) false false))))